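; Quest trigger volume that flags itself as activated when the third-person player character is inside its box.
; While enabled and not yet activated, it polls every Tick with a box overlap query sized to its Collision component, rather than using overlap events.
; Activated latches until Deactivate clears it, with simple functions exposed to set or clear both the Enabled and Activated flags.
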(event `self.ReceiveTick`
  (params (DeltaSeconds :type "Float (single-precision)"))
  (if (`self.Enabled`)
    (if (not (`self.Activated`))
      (bind (_outactors _returnvalue) (`KismetSystemLibrary.BoxOverlapActors` (`SceneComponent.K2_GetComponentLocation` (`self.Collision`)) (`BoxComponent.GetScaledBoxExtent` (`self.Collision`)) (`|MakeArray` "ObjectTypeQuery3" :!type "EObjectTypeQuery Enum") "/Game/_GameManager/BP_ThirdPersonCharacter.BP_ThirdPersonCharacter_C"))
      (if _returnvalue
        (set `self.Activated` true)))))

(fn `Activate`
  (set `self.Activated` true))

(fn `Deactivate`
  (set `self.Activated` false))

(fn `Disable`
  (set `self.Enabled` false))

(fn `Enable`
  (set `self.Enabled` true))

(fn `UserConstructionScript`)