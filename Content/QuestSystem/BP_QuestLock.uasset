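; BP_QuestLock is a quest-system actor that acts as a switchable lock by toggling the collision of its Collision component.
; Enable and Disable set the Enabled flag and switch that component between query-and-physics collision and no collision.
; BeginPlay calls whichever function matches the initial flag, so the collision state follows Enabled when play starts.
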(event `self.ReceiveBeginPlay`
  (if (`self.Enabled`)
    (`self.Enable`)
    (else
      (`self.Disable`))))

(fn `Disable`
  (set `self.Enabled` false)
  (`PrimitiveComponent.SetCollisionEnabled` (`self.Collision`) "NoCollision"))

(fn `Enable`
  (set `self.Enabled` true)
  (`PrimitiveComponent.SetCollisionEnabled` (`self.Collision`) "QueryAndPhysics"))

(fn `UserConstructionScript`)