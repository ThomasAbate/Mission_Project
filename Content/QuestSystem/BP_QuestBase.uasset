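; Base quest actor that tracks a list of typed objectives (interact, follow, kill, fetch, exit) for an owning character.
; StartQuest finds the BP_EventDispatcher and subscribes to events for every objective type except exit.
; Events involving the owner update progress on objectives matching type and target class or actor, optionally in order.
; Completion follows the last objective when ordered; unordered quests only clear the flag on incomplete objectives.
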(event `self.ReceiveBeginPlay`)

(event `/Game/Event/BPI_EventSubscribable.ReceiveNewEvent`
  (params (Event :type "/Game/Event/SEvent Structure"))
  (bind (_type _pickup _triggeractor _otheractor _change) (break `/Game/Event/SEvent` Event))
  (if (== (`self.OwnerChar`) _otheractor)
    (switch `/Game/Event/EEvent` _type
      (:`NewEnumerator1`
        (`self.OnNotifie` "NewEnumerator2" _triggeractor _change))
      (:`NewEnumerator2`
        (`self.OnNotifie` "NewEnumerator3" _triggeractor _change))
      (:`NewEnumerator3`
        (`self.OnNotifie` "NewEnumerator1" _triggeractor _change))
      (:`NewEnumerator4`
        (`self.OnNotifie` "NewEnumerator0" _triggeractor _change))
      (:`NewEnumerator5`
        (`self.OnNotifie` "NewEnumerator4" _triggeractor)))))

(fn `OnEndNotifie`
  (bind _objectives (`self.Objectives`))
  (if (`self.IsOrdered`)
    (set `self.IsQuestComplete` (`.IsComplete_20_8C0348CA4DC18C03D8ACB98DB195B7DE` (break `/Game/QuestSystem/SQuestObjective` (`|GetArrayItem` _objectives (- (`KismetArrayLibrary.Array_Length` _objectives) 1)))))
    (else
      (for _array_element _objectives
        (if (not (`.IsComplete_20_8C0348CA4DC18C03D8ACB98DB195B7DE` (break `/Game/QuestSystem/SQuestObjective` _array_element)))
          (set `self.IsQuestComplete` false)
          (break))))))

(fn `OnNotifie`
  (params (Type :type "/Game/QuestSystem/EQuestObjectives Enum" :default "NewEnumerator0") (TriggerActor :type "Actor Object Reference") (NumberChange :type Integer))
  (for _array_element (`self.Objectives`)
    (bind (_type _targetactor _targetclass _numbertocomplete _currentnumber _targetisclass _iscomplete) (break `/Game/QuestSystem/SQuestObjective` _array_element))
    (if (`|EnumEquality` Type _type)
      (if _targetisclass
        (if (== (`GameplayStatics.GetObjectClass` TriggerActor) _targetclass)
          (bind _returnvalue (+ _currentnumber NumberChange))
          (`|VariableSetRef` _currentnumber _returnvalue :!label _label)
          (`|VariableSetRef` _iscomplete (== _returnvalue _numbertocomplete))
          (if (and (`self.IsOrdered`) (not _iscomplete)) :!label _label_2
            (break)))
        (elif (== _targetactor TriggerActor)
          (goto _label)))
      (else
        (goto _label_2))))
  (`self.OnEndNotifie`))

(fn `StartQuest`
  (params (Owner :type "/Game/_GameManager/BP_ThirdPersonCharacter Object Reference"))
  (set `self.OwnerChar` Owner)
  (bind _returnvalue (`GameplayStatics.GetActorOfClass` "/Game/Event/BP_EventDispatcher.BP_EventDispatcher_C"))
  (set `self.Notifier` _returnvalue)
  (for _array_element (`self.Objectives`)
    (switch `/Game/QuestSystem/EQuestObjectives` (`.Type_2_8ECC82CE4A362874F0ED01872763A235` (break `/Game/QuestSystem/SQuestObjective` _array_element))
      (:`NewEnumerator0`
        (`/Game/Event/BP_EventDispatcher.Subscribe` (`self.Notifier`) "NewEnumerator4" self))
      (:`NewEnumerator1`
        (`/Game/Event/BP_EventDispatcher.Subscribe` (`self.Notifier`) "NewEnumerator3" self))
      (:`NewEnumerator2`
        (`/Game/Event/BP_EventDispatcher.Subscribe` (`self.Notifier`) "NewEnumerator1" self))
      (:`NewEnumerator3`
        (`/Game/Event/BP_EventDispatcher.Subscribe` (`self.Notifier`) "NewEnumerator2" self)))))

(fn `UserConstructionScript`)