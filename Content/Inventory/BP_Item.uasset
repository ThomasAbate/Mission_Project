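; BP_Item is an inventory item actor that can be picked up and counted in an owner's inventory.
; Add and remove functions adjust the count at the item's ID in the owner's InventoryArray and record the change through the owner's EventDispatch.
; Adding also moves the actor to a fixed location below the world origin.
; Pickup prints a message, triggers a briefly delayed self-destruct and returns the Item value.
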(event `Destory Item`
  (`KismetSystemLibrary.Delay` 0.1)
  (`self.K2_DestroyActor`))

(fn `AddToInventory`
  (params (Owner :type "/Game/_GameManager/BP_ThirdPersonCharacter Object Reference"))
  (`/Engine/EditorBlueprintResources/StandardMacros.IncrementInt` (`.Number_4_40AE9B2E495F023C3B9DCA8B3AC86782` (break `/Game/Inventory/SInventorySlot` (`|GetArrayItem` (`/Game/_GameManager/BP_ThirdPersonCharacter.InventoryArray` Owner) (`self.ID`))))
    (:`  `
      (`/Game/Event/BP_EventDispatcher.Record` (`/Game/_GameManager/BP_ThirdPersonCharacter.EventDispatch` Owner) (make `/Game/Event/SEvent` "NewEnumerator4" (struct) self Owner 1))
      (`self.K2_SetActorLocation` (0.0 0.0 -50.0)))))

(fn `Pick Up Item`
  (returns (item :type String))
  (`KismetSystemLibrary.PrintString` "Item Picked Up")
  (`self.Destory Item`)
  (return (`self.item`)))

(fn `RemoveFromInventory`
  (params (Owner :type "/Game/_GameManager/BP_ThirdPersonCharacter Object Reference"))
  (`/Engine/EditorBlueprintResources/StandardMacros.DecrementInt` (`.Number_4_40AE9B2E495F023C3B9DCA8B3AC86782` (break `/Game/Inventory/SInventorySlot` (`|GetArrayItem` (`/Game/_GameManager/BP_ThirdPersonCharacter.InventoryArray` Owner) (`self.ID`))))
    (:`  `
      (`/Game/Event/BP_EventDispatcher.Record` (`/Game/_GameManager/BP_ThirdPersonCharacter.EventDispatch` Owner) (make `/Game/Event/SEvent` "NewEnumerator4" (struct) self Owner -1)))))

(fn `UserConstructionScript`)