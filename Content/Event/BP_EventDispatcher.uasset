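; BP_EventDispatcher routes game events to subscribers by type and manages an on-screen message log through WBP_EventLog.
; Subscribe registers listeners in a map keyed by event type, and Record forwards each event to that type's listeners via ReceiveNewEvent.
; Separately, Log shows messages up to a line limit and queues overflow.
; Tick periodically drops the oldest line, promotes a queued one, and refreshes the widget every frame.
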(event `self.ReceiveBeginPlay`
  (bind _returnvalue (`|CreateWidget` "/Game/Event/WBP_EventLog.WBP_EventLog_C"))
  (bind _output_get (set `self.Widget` _returnvalue))
  (`UserWidget.AddToViewport` _output_get 0))

(event `self.ReceiveTick`
  (params (DeltaSeconds :type "Float (single-precision)"))
  (bind _output_get (set `self.Timer` (+ DeltaSeconds (`self.Timer`))))
  (if (>= _output_get (`self.Time`))
    (set `self.Timer` 0.0)
    (if (`KismetArrayLibrary.Array_IsNotEmpty` (`self.Logged`))
      (`KismetArrayLibrary.Array_Remove` (`self.Logged`))
      (if (`KismetArrayLibrary.Array_IsNotEmpty` (`self.Queued`))
        (`KismetArrayLibrary.Array_Add` (`self.Logged`) (`|GetArrayItem` (`self.Queued`)))
        (`KismetArrayLibrary.Array_Remove` (`self.Queued`))
        (`self.Bind`)
        (else
          (`self.Bind`)))
      (else
        (`self.Bind`)))
    (else
      (`self.Bind`))))

(fn `Bind`
  (`/Game/Event/WBP_EventLog.Log` (`self.Widget`) (`self.Logged`)))

(fn `Log`
  (params (Message :type Text))
  (if (< (`KismetArrayLibrary.Array_Length` (`self.Logged`)) (`self.Lines`))
    (`KismetArrayLibrary.Array_Add` (`self.Logged`) Message)
    (`self.Bind`)
    (else
      (`KismetArrayLibrary.Array_Add` (`self.Queued`) Message))))

(fn `Record`
  (params (Event :type "/Game/Event/SEvent Structure"))
  (bind (_value _returnvalue) (`BlueprintMapLibrary.Map_Find` (`self.Subscribers`) (`.Type_9_51B24EC54FAC835ABD96C39D6F5A4262` (break `/Game/Event/SEvent` Event))))
  (if _returnvalue
    (for _array_element (break `/Game/Event/SEventSubscribers` _value)
      (`/Game/Event/BPI_EventSubscribable.ReceiveNewEvent` _array_element Event))))

(fn `Subscribe`
  (params (Event :type "/Game/Event/EEvent Enum" :default "NewEnumerator0") (`Subscriber ` :type "/Game/Event/BPI_EventSubscribable Interface"))
  (if (`BlueprintMapLibrary.Map_Contains` (`self.Subscribers`) Event)
    (`KismetArrayLibrary.Array_AddUnique` (break `/Game/Event/SEventSubscribers` (`BlueprintMapLibrary.Map_Find` (`self.Subscribers`) Event)) `Subscriber `)
    (else
      (`BlueprintMapLibrary.Map_Add` (`self.Subscribers`) Event (make `/Game/Event/SEventSubscribers` (`|MakeArray` `Subscriber `))))))

(fn `UserConstructionScript`)