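; BP_NPC is a quest-giver NPC that steps through an array of quests, each with its own dialogue.
; Interact records a quest event, then after a short delay either starts and logs the current quest or picks dialogue by its status.
; A completed quest advances the index to the next one.
; HIt reduces Health when damage is allowed; an AI move toward the player is left unconnected.
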(event `HIt`
  (if (`self.CanBeDamaged`)
    (set `self.Health` (- (`self.Health`) (`KismetStringLibrary.Conv_StringToInt` "Player damage")))))

(event `self.ReceiveTick`
  (params (DeltaSeconds :type "Float (single-precision)")))

(event `Interact`
  (params (OtherActor :type "Actor Object Reference"))
  (bind _asbp_third_person_character (cast `/Game/_GameManager/BP_ThirdPersonCharacter` OtherActor :!pure true))
  (bind _currentquest (`self.CurrentQuest`))
  (bind (_prequestdialogue _activequestdialogue _postquestdialogue) (break `/Game/QuestSystem/SNPCQuestAssets` (`|GetArrayItem` (`self.Quests`) (`self.CurrentQuest`))))
  (bind (_prequestdialogue_2 _activequestdialogue_2 _postquestdialogue_2 _questobject) (break `/Game/QuestSystem/SNPCQuestAssets` (`|GetArrayItem` (`self.Quests`) (`self.CurrentQuest`))))
  (`/Game/Event/BP_EventDispatcher.Record` (`/Game/QuestSystem/BP_QuestBase.Notifier` (`.QuestObject_12_28871CA041D7D562F7F5B899DD064063` (break `/Game/QuestSystem/SNPCQuestAssets` (`|GetArrayItem` (`self.Quests`) (`self.CurrentQuest`))))) (make `/Game/Event/SEvent` "NewEnumerator1" (struct) self OtherActor))
  (`KismetSystemLibrary.Delay` 0.2)
  (if (`KismetArrayLibrary.Array_Contains` (`/Game/_GameManager/BP_ThirdPersonCharacter.QuestLog` (cast `/Game/_GameManager/BP_ThirdPersonCharacter` (`Controller.K2_GetPawn` (`GameplayStatics.GetPlayerController` 0)) :!pure true)) _questobject)
    (switch `/Game/QuestSystem/EQuestStatus` (`/Game/QuestSystem/BP_QuestBase.Status` _questobject)
      (:`NewEnumerator0`
        (set `self.CurrentDialogue` _activequestdialogue))
      (:`NewEnumerator1`
        (set `self.CurrentDialogue` _postquestdialogue)
        (if (< _currentquest (- (`KismetArrayLibrary.Array_Length` (`self.Quests`)) 1))
          (`/Engine/EditorBlueprintResources/StandardMacros.IncrementInt` _currentquest))))
    (else
      (set `self.CurrentDialogue` _prequestdialogue_2)
      (`KismetArrayLibrary.Array_Add` (`/Game/_GameManager/BP_ThirdPersonCharacter.QuestLog` _asbp_third_person_character) _questobject)
      (`/Game/QuestSystem/BP_QuestBase.StartQuest` _questobject _asbp_third_person_character))))

(fn `UserConstructionScript`)